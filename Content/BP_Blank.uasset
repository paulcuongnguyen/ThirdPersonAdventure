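; BP_Blank is a damageable plank actor made of static meshes that collapses when its HP runs out.
; AnyDamage subtracts from HP, and Tick writes the value to the PlankHP text component every frame.
; At zero or below, a DoOnce enables physics on six meshes, destroys the text, then switches physics off after a delay to freeze the pieces.
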(event EventBeginPlay)

(event Collision|EventActorBeginOverlap
  (params (OtherActor :type Actor%20Object%20Reference)))

(event EventTick
  (params (DeltaSeconds :type Float%20%28single-precision%29))
  (bind _plank_hp (Variables|Default|GetPlank_HP))
  (bind _plank_hp_2 (Variables|Default|GetPlank_HP))
  (if (Utilities|IsValid _plank_hp_2)
    (Rendering|Components|TextRender|SetText _plank_hp_2 (Utilities|Text|ToText(String) (Utilities|String|Append "HP: " (Utilities|String|ToString(Text) (Utilities|Text|ToText(Float) (Variables|Default|GetHP) "HalfToEven"))))))
  (if (<= (Variables|Default|GetHP) 0.0)
    (Utilities|FlowControl|DoOnce false
      (:Completed
        (Physics|SetSimulatePhysics (Variables|Debug|GetStaticMeshComponent) true)
        (if (Utilities|IsValid _plank_hp)
          (Components|DestroyComponent _plank_hp)
          (Utilities|FlowControl|Delay 5.0)
          (Physics|SetSimulatePhysics (Variables|Debug|GetStaticMeshComponent) false))))))

(event Game|Damage|EventAnyDamage
  (params (Damage :type Float%20%28single-precision%29) (DamageType :type Damage%20Type%20Object%20Reference) (InstigatedBy :type Controller%20Object%20Reference) (DamageCauser :type Actor%20Object%20Reference))
  (Variables|Default|SetHP (- (Variables|Default|GetHP) Damage)))

(fn ConstructionScript)