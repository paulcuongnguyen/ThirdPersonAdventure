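; An explosive barrel actor that catches fire when it takes any damage, then explodes.
; AnyDamage attaches fire particles and sound to the mesh, waits through a short Delay, then spawns the explosion effect, sound and world camera shake.
; Radial damage with falloff radiates from the Epicenter component before the actor destroys itself.
; No guard blocks repeat hits, so further damage during the delay adds more fire effects.
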(event EventBeginPlay)

(event Collision|EventActorBeginOverlap
  (params (OtherActor :type Actor%20Object%20Reference)))

(event EventTick
  (params (DeltaSeconds :type Float%20%28single-precision%29)))

(event Game|Damage|EventAnyDamage
  (params (Damage :type Float%20%28single-precision%29) (DamageType :type Damage%20Type%20Object%20Reference) (InstigatedBy :type Controller%20Object%20Reference) (DamageCauser :type Actor%20Object%20Reference))
  (bind _returnvalue (Transformation|GetActorLocation))
  (bind _staticmeshcomponent (Variables|Debug|GetStaticMeshComponent))
  (Effects|SpawnEmitterAttached "/Game/StarterContent/Particles/P_Fire.P_Fire" _staticmeshcomponent "None")
  (Audio|SpawnSoundAttached "/Game/StarterContent/Audio/Fire_Sparks01.Fire_Sparks01" _staticmeshcomponent "None" "0, 0, 0" "0, 0, 0" "KeepRelativeOffset" true 1.0 1.0 0.0 0 0)
  (Utilities|FlowControl|Delay 2.0)
  (Effects|SpawnEmitteratLocation "/Game/StarterContent/Particles/P_Explosion.P_Explosion" _returnvalue "0, 0, 0" "3.000000,3.000000,3.000000")
  (Audio|PlaySoundatLocation "/Game/StarterContent/Audio/Explosion01.Explosion01" _returnvalue "0, 0, 0" 1.0 1.0 0.0 0 0 0 0)
  (Camera|PlayWorldCameraShake "/Game/BP_CamShake1.BP_CamShake1_C" _returnvalue 0.0 5e+04)
  (Class|GameplayStatics|ApplyRadialDamagewithFalloff 1e+02 1e+01 (Transformation|GetWorldLocation (Variables|Default|GetEpicenter)) 0.0 5e+02 0.0 0 0 0 0 "ECC_Visibility")
  (Actor|DestroyActor))

(fn ConstructionScript)