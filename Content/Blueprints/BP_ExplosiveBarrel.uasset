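; Explosive barrel actor that catches fire when it takes any damage, then explodes a few seconds later.
; AnyDamage attaches fire and sound to the Epicenter component, then after delays spawns FS_MasterField1 there, followed by explosion effects and a world camera shake.
; The blast applies radial damage with falloff before the barrel destroys itself.
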(event EventBeginPlay)

(event Collision|EventActorBeginOverlap
  (params (OtherActor :type Actor%20Object%20Reference)))

(event EventTick
  (params (DeltaSeconds :type Float%20%28single-precision%29)))

(event Game|Damage|EventAnyDamage
  (params (Damage :type Float%20%28single-precision%29) (DamageType :type Damage%20Type%20Object%20Reference) (InstigatedBy :type Controller%20Object%20Reference) (DamageCauser :type Actor%20Object%20Reference))
  (bind _returnvalue (Transformation|GetActorLocation))
  (bind _epicenter (Variables|Default|GetEpicenter))
  (bind _returnvalue_2 (Transformation|GetWorldLocation _epicenter))
  (Development|PrintString "Barrel damaged")
  (Effects|SpawnEmitterAttached "/Game/StarterContent/Particles/P_Fire.P_Fire" _epicenter "None")
  (Audio|SpawnSoundAttached "/Game/StarterContent/Audio/Fire_Sparks01.Fire_Sparks01" _epicenter "None" "0, 0, 0" "0, 0, 0" "KeepRelativeOffset" true 1.0 1.0 0.0 0 0)
  (Utilities|FlowControl|Delay 2.0)
  (Game|SpawnActorfromClass "/Game/FS_MasterField1.FS_MasterField1_C" (Math|Conversions|ToTransform(Vector) _returnvalue_2) "Undefined" "MultiplyWithRoot" 0 0)
  (Utilities|FlowControl|Delay 1.0)
  (Effects|SpawnEmitteratLocation "/Game/StarterContent/Particles/P_Explosion.P_Explosion" _returnvalue_2 "0, 0, 0" "3.000000,3.000000,3.000000")
  (Audio|PlaySoundatLocation "/Game/StarterContent/Audio/Explosion01.Explosion01" _returnvalue "0, 0, 0" 1.0 1.0 0.0 0 0 0 0)
  (Camera|PlayWorldCameraShake "/Game/Blueprints/BP_CamShake1.BP_CamShake1_C" _returnvalue 0.0 5e+04)
  (Class|GameplayStatics|ApplyRadialDamagewithFalloff 1e+02 1e+01 _returnvalue_2 0.0 1e+03 0.0 0 0 0 0 "ECC_Visibility")
  (Actor|DestroyActor))

(fn ConstructionScript)