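; Explosive projectile that deals heavy damage to any BP_ThirdPersonCharacter overlapping its Sphere, ignoring all other actors.
; On such a hit it applies damage and launches the character mesh with a fixed upward impulse on the pelvis bone at the Bullet's location.
; It then spawns an explosion effect and sound there and destroys itself.
; A directional knockback calculation sits unused in the graph.
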(event OnComponentBeginOverlap(Sphere)
  (params (OverlappedComponent :type Primitive%20Component%20Object%20Reference) (OtherActor :type Actor%20Object%20Reference) (OtherComp :type Primitive%20Component%20Object%20Reference) (OtherBodyIndex :type Integer) (bFromSweep :type Boolean) (SweepResult :type Hit%20Result%20Structure%20%28by%20ref%29))
  (bind _bullet (Variables|Default|GetBullet))
  (bind _returnvalue (Transformation|GetWorldLocation _bullet))
  (bind _asbp_third_person_character (Utilities|Casting|CastToBP_ThirdPersonCharacter OtherActor))
  (Game|Damage|ApplyDamage OtherActor 1e+02 0 0)
  (Physics|AddImpulseatLocation (Variables|/Script/Engine.Character|GetMesh _asbp_third_person_character) "0.000000,0.000000,35000.000000" _returnvalue "pelvis")
  (Effects|SpawnEmitteratLocation "/Game/StarterContent/Particles/P_Explosion.P_Explosion" _returnvalue "0, 0, 0" "3.000000,3.000000,3.000000")
  (Audio|PlaySoundatLocation "/Game/StarterContent/Audio/Explosion01.Explosion01" _returnvalue "0, 0, 0" 1.0 1.0 0.0 0 0 0 0)
  (Actor|DestroyActor))

(event EventBeginPlay)

(event EventTick
  (params (DeltaSeconds :type Float%20%28single-precision%29)))

(fn ConstructionScript)